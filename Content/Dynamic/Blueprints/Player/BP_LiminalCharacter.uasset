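; Player character Blueprint that handles surface-dependent footstep sounds.
; Move input plays FootstepsTL while the character moves on the ground and stops it on release.
; FootstepTry calls TraceFootsteps, which sphere-traces to the capsule's base and plays office floor, stone or ceramic sounds by physical surface.
; The graph shows no live link from FootstepsTL to FootstepTry; an older timeline hookup and timer logic sit unreachable.
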(event `EnhancedInput|/Game/Dynamic/Blueprints/Player/Inputs/IA_Move`
  (params (ActionValue :type "Vector2D Structure") (ElapsedSeconds :type "Float (double-precision)") (TriggeredSeconds :type "Float (double-precision)") (InputAction :type "InputAction Object Reference" :default "/Game/Dynamic/Blueprints/Player/Inputs/IA_Move.IA_Move"))
  ;[1 1 1] Footsteps
  (:`Triggered`
    (if (> (`KismetMathLibrary.VSize` (`self.GetVelocity`)) 0.0)
      (if (not (`NavMovementComponent.IsFalling` (`self.CharacterMovement`)))
        (`TimelineComponent.Play` (`self.Footsteps_TL`)))))
  (:`Completed`
    (`TimelineComponent.Stop` (`self.Footsteps_TL`))))

(event `CheckIfStops`)

(fn `FootstepTry`
  (`self.TraceFootsteps`))

(fn `TraceFootsteps`
  (bind _returnvalue (`self.K2_GetActorLocation`))
  (bind _capsulecomponent (`self.CapsuleComponent`))
  (bind (_outhit _returnvalue_2) (`KismetSystemLibrary.SphereTraceSingle` _returnvalue (`KismetMathLibrary.MakeVector` (.x _returnvalue) (.y _returnvalue) (- (.z _returnvalue) (`CapsuleComponent.GetScaledCapsuleHalfHeight` _capsulecomponent))) (`CapsuleComponent.GetScaledCapsuleRadius` _capsulecomponent) "TraceTypeQuery1"))
  (if _returnvalue_2
    (switch `EPhysicalSurface` (`GameplayStatics.GetSurfaceType` _outhit)
      (:`SurfaceType1`
        (bind (_bblockinghit _binitialoverlap _time _distance _location) (`GameplayStatics.BreakHitResult` _outhit))
        (`GameplayStatics.PlaySoundAtLocation` "/Game/Static/Sounds/Footsteps/OfficeFloor/SC_FloorStep.SC_FloorStep" _location (struct) 1.0 1.0 0.0 null null null null))
      (:`SurfaceType2`
        (`GameplayStatics.PlaySoundAtLocation` "/Game/Static/Sounds/Footsteps/Stone/SC_StepStone.SC_StepStone" _location (struct) 1.0 1.0 0.0 null null null null))
      (:`SurfaceType3`
        (`GameplayStatics.PlaySoundAtLocation` "/Game/Static/Sounds/Footsteps/CeramicPlate/SC_PlateStep.SC_PlateStep" _location (struct) 1.0 1.0 0.0 null null null null)))))

(fn `UserConstructionScript`)